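; Player character for the maze/mansion game, handling input, interaction, melee combat, health and a two-slot inventory.
; Input drives camera and MovementComp, while capsule overlaps notify interactables through an interface and the Interact key triggers overlapping items.
; Escape, M or the menu's Continue toggle pause, using cursor visibility as state.
; Construction sockets HZ body-part components, attacks play random armed/unarmed montages, and damage updates StatsComp, signalling death at zero.
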(event OnComponentBeginOverlap(CapsuleComponent)
  (params (OverlappedComponent :type Primitive%20Component%20Object%20Reference) (OtherActor :type Actor%20Object%20Reference) (OtherComp :type Primitive%20Component%20Object%20Reference) (OtherBodyIndex :type Integer) (bFromSweep :type Boolean) (SweepResult :type Hit%20Result%20Structure%20%28by%20ref%29))
  ;[1 1 1] Interaction Interface - On range entered
  (if (Utilities|DoesObjectImplementInterface OtherActor "/Game/Items/interaction_interface.interaction_interface_C")
    (Class|InteractionInterface|OnRangeEntered(Message) OtherActor self)))

(event OnComponentEndOverlap(CapsuleComponent)
  (params (OverlappedComponent :type Primitive%20Component%20Object%20Reference) (OtherActor :type Actor%20Object%20Reference) (OtherComp :type Primitive%20Component%20Object%20Reference) (OtherBodyIndex :type Integer))
  ;[1 1 1] Interaction Interface - On range exit
  (if (Utilities|DoesObjectImplementInterface OtherActor "/Game/Items/interaction_interface.interaction_interface_C")
    (Class|InteractionInterface|RangeExit(Message) OtherActor)))

(event Custom|Continue
  (bind _returnvalue (Game|GetPlayerController 0))
  (bind _menu (Variables|Default|GetMenu))
  (bind _hud (Variables|Default|GetHUD))
  ;[1 1 1] PuaseMenuActions
  (if (not (Variables|/Script/Engine.PlayerController|GetbShowMouseCursor (Game|GetPlayerController 0)))
    (UserInterface|Viewport|AddtoViewport _menu 0)
    (Variables|/Script/Engine.PlayerController|SetbShowMouseCursor _returnvalue true)
    (Input|SetInputModeGameandUI _returnvalue 0 "DoNotLock" true)
    (Widget|SetVisibility _hud "Hidden")
    (Game|SetGamePaused true)
    (else
      (Widget|RemovefromParent _menu)
      (Variables|/Script/Engine.PlayerController|SetbShowMouseCursor _returnvalue false)
      (Input|SetInputModeGameOnly _returnvalue)
      (Widget|SetVisibility _hud "Visible")
      (Game|SetGamePaused false))))

(event EventBeginPlay
  (CallFunction|SetUpWidgets)
  (EventDispatchers|BindEventtoContinue (Variables|Default|GetMenu) (delegate Custom|Continue)))

(event Input|ActionEvents|InputActionInteract
  (params (Key :type Key%20Structure :default "None"))
  ;[1 1 1] Press the key to interact
  (:Pressed
    (bind _array_element (Utilities|Array|ForEachLoopwithBreak (Collision|GetOverlappingActors (Variables|Default|GetCapsuleComponent) "/Game/Items/InteractiveItem.InteractiveItem_C" :!class /Script/Engine.PrimitiveComponent))
      (:LoopBody
        (Class|InteractionInterface|OnInteracted(Message) _array_element)))))

(event Input|AxisEvents|InputAxisWalkForward/Backward
  (params (AxisValue :type Float%20%28single-precision%29))
  ;[1 1 1] Movement
  (Default|MoveForward/Back (Variables|Default|GetMovementComp) AxisValue))

(event Input|AxisEvents|InputAxisWalkLeft/Right
  (params (AxisValue :type Float%20%28single-precision%29))
  ;[1 1 1] Movement
  (Default|MoveLeft/Right (Variables|Default|GetMovementComp) AxisValue))

(event Input|AxisEvents|InputAxisLookUp/Down
  (params (AxisValue :type Float%20%28single-precision%29))
  ;[1 1 1] Camera Control
  (Pawn|Input|AddControllerPitchInput AxisValue))

(event Input|AxisEvents|InputAxisLookLeft/Right
  (params (AxisValue :type Float%20%28single-precision%29))
  ;[1 1 1] Camera Control
  (Pawn|Input|AddControllerYawInput AxisValue))

(event Input|KeyboardEvents|M
  (params (Key :type Key%20Structure :default "None"))
  (bind _returnvalue (Game|GetPlayerController 0))
  (bind _menu (Variables|Default|GetMenu))
  (bind _hud (Variables|Default|GetHUD))
  ;[1 1 1] PuaseMenuActions
  (:Pressed
    (if (not (Variables|/Script/Engine.PlayerController|GetbShowMouseCursor (Game|GetPlayerController 0)))
      (UserInterface|Viewport|AddtoViewport _menu 0)
      (Variables|/Script/Engine.PlayerController|SetbShowMouseCursor _returnvalue true)
      (Input|SetInputModeGameandUI _returnvalue 0 "DoNotLock" true)
      (Widget|SetVisibility _hud "Hidden")
      (Game|SetGamePaused true)
      (else
        (Widget|RemovefromParent _menu)
        (Variables|/Script/Engine.PlayerController|SetbShowMouseCursor _returnvalue false)
        (Input|SetInputModeGameOnly _returnvalue)
        (Widget|SetVisibility _hud "Visible")
        (Game|SetGamePaused false)))))

(event Input|KeyboardEvents|Escape
  (params (Key :type Key%20Structure :default "None"))
  (bind _returnvalue (Game|GetPlayerController 0))
  (bind _menu (Variables|Default|GetMenu))
  (bind _hud (Variables|Default|GetHUD))
  ;[1 1 1] PuaseMenuActions
  (:Pressed
    (if (not (Variables|/Script/Engine.PlayerController|GetbShowMouseCursor (Game|GetPlayerController 0)))
      (UserInterface|Viewport|AddtoViewport _menu 0)
      (Variables|/Script/Engine.PlayerController|SetbShowMouseCursor _returnvalue true)
      (Input|SetInputModeGameandUI _returnvalue 0 "DoNotLock" true)
      (Widget|SetVisibility _hud "Hidden")
      (Game|SetGamePaused true)
      (else
        (Widget|RemovefromParent _menu)
        (Variables|/Script/Engine.PlayerController|SetbShowMouseCursor _returnvalue false)
        (Input|SetInputModeGameOnly _returnvalue)
        (Widget|SetVisibility _hud "Visible")
        (Game|SetGamePaused false)))))

(fn ConstructionScript
  (Transformation|AttachComponentToComponent (Variables|Default|GetHeadHZ) (Variables|Character|GetMesh) "Head" "KeepRelative" "KeepRelative" "KeepRelative" true)
  (Transformation|AttachComponentToComponent (Variables|Default|GetBodyHZ) (Variables|Character|GetMesh) "Spine" "KeepRelative" "KeepRelative" "KeepRelative" true)
  (Transformation|AttachComponentToComponent (Variables|Default|GetLArmHZ) (Variables|Character|GetMesh) "LeftArm" "KeepRelative" "KeepRelative" "KeepRelative" true)
  (Transformation|AttachComponentToComponent (Variables|Default|GetRArmHZ) (Variables|Character|GetMesh) "RightArm" "KeepRelative" "KeepRelative" "KeepRelative" true))

(fn UpdateHealthFunc
  (params (Damage :type Float%20%28single-precision%29))
  (bind _statscomp (Variables|Default|GetStatsComp))
  (bind _output_get (Variables|/Game/Character/MazeCharacter/StatsComp.StatsComp_C|SetHealth _statscomp (- (Variables|/Game/Character/MazeCharacter/StatsComp.StatsComp_C|GetHealth _statscomp) Damage)))
  (Default|CallHealthUpdated _output_get)
  (if (<= (Variables|/Game/Character/MazeCharacter/StatsComp.StatsComp_C|GetHealth (Variables|Default|GetStatsComp)) 0.0)
    (Default|CallDie)))

(fn Attack
  (params (Time :type Float%20%28single-precision%29))
  (if (Variables|Default|GetbIsArmed)
    (Animation|PlayAnimMontage (Utilities|Select :Index (Math|Random|RandomInteger 2) :Option%200 "/Game/Character/MazeCharacter/Anims/Attacks/Mannequin_Stabbing1_Montage.Mannequin_Stabbing1_Montage" :Option%201 "/Game/Character/MazeCharacter/Anims/Attacks/Mannequin_Standing_Melee_Punch_Montage.Mannequin_Standing_Melee_Punch_Montage") 1.0 "None")
    (else
      (Animation|PlayAnimMontage (Utilities|Select :Index (Math|Random|RandomInteger 3) :Option%200 "/Game/Character/MazeCharacter/Anims/Attacks/Manneequin_Elbow_Uppercut_Combo_Montage.Manneequin_Elbow_Uppercut_Combo_Montage" :Option%201 "/Game/Character/MazeCharacter/Anims/Attacks/Mannequin_Cross_Punch_Montage.Mannequin_Cross_Punch_Montage" :Option%202 "/Game/Character/MazeCharacter/Anims/Attacks/Mannequin_Standing_Melee_Punch_Montage.Mannequin_Standing_Melee_Punch_Montage") 1.0 "None"))))

(fn PickUpItem
  (params (Item :type Interactive%20Item%20Object%20Reference))
  (Utilities|IsValid (Variables|Default|GetItemOne)
    (:Is%20Valid
      (Utilities|IsValid (Variables|Default|GetItemTwo)
        (:Is%20Valid)
        (:Is%20Not%20Valid
          (Variables|Default|SetItemTwo Item))))
    (:Is%20Not%20Valid
      (Variables|Default|SetItemOne Item)))
  (CallFunction|UpdateItemAttachments))

(fn UpdateItemAttachments
  (bind _itemone (Variables|Default|GetItemOne))
  (bind _itemtwo (Variables|Default|GetItemTwo))
  (Utilities|FlowControl|Sequence
    (:then_0
      (Utilities|IsValid _itemone
        (:Is%20Valid
          (Transformation|AttachComponentToComponent _itemone (Variables|Character|GetMesh) "MainSocket" "SnapToTarget" "SnapToTarget" "SnapToTarget" true)
          (Variables|/Game/Items/InteractiveItem.InteractiveItem_C|SetbIsEquipped _itemone true))))
    (:then_1
      (Utilities|IsValid _itemtwo
        (:Is%20Valid
          (Transformation|AttachComponentToComponent _itemtwo (Variables|Character|GetMesh) "SecondarySocket" "SnapToTarget" "SnapToTarget" "SnapToTarget" true)
          (Variables|/Game/Items/InteractiveItem.InteractiveItem_C|SetbIsEquipped _itemtwo true))))))

(fn SetUpWidgets
  (bind _returnvalue (UserInterface|CreateWidget "/Game/UI/HUD.HUD_C" (Game|GetPlayerController 0)))
  (bind _output_get (Variables|Default|SetHUD _returnvalue))
  (UserInterface|Viewport|AddtoViewport _output_get 0)
  (bind _returnvalue_2 (UserInterface|CreateWidget "/Game/UI/PauseMenu.PauseMenu_C" (Game|GetPlayerController 0)))
  (Variables|Default|SetMenu _returnvalue_2)
  (Input|SetInputModeGameOnly (Game|GetPlayerController 0)))