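; Player hero character with camera-relative movement, stamina-limited sprinting, unarmed-only jumping and melee combat, reporting noise as it walks.
; A key toggles between spawned Knife and Punch weapon actors attached at a socket.
; A profiling timer measures attack hold time, which combines with kill streak and armed state into an AttackType bitmask.
; Attacks turn toward an overlapped NPC inside its attack area, play a montage and block movement input until a delay ends.
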(event EventTick
  (params (DeltaSeconds :type Float%20%28single-precision%29))
  ;[1 1 1] Every Second
  (Utilities|CalculateStamina))

(event Collision|EventActorBeginOverlap
  (params (OtherActor :type Actor%20Object%20Reference))
  ;[1 1 1] Overlapped Item
  (Variables|Default|SetOverlappedActor OtherActor))

(event Collision|EventActorEndOverlap
  (params (OtherActor :type Actor%20Object%20Reference))
  ;[1 1 1] Overlapped Item
  (Variables|Default|SetOverlappedActor 0))

(event EventBeginPlay
  (|CallParentFunction))

(event Input|ActionEvents|InputActionAttack
  (params (Key :type Key%20Structure :default "None"))
  ;[1 1 1] Attack
  (:Pressed
    (Class|KismetAnimationLibrary|StartProfilingTimer))
  (:Released
    (bind _returnvalue (Class|KismetAnimationLibrary|EndProfilingTimer true))
    (Utilities|Attack _returnvalue)))

(event Input|ActionEvents|InputActionSprint
  (params (Key :type Key%20Structure :default "None"))
  ;[1 1 1] Sprint
  (:Pressed
    (if (>= (Variables|Default|GetStamina) 0.0)
      (Variables|Default|SetbRunning true)
      (Variables|/Script/Engine.CharacterMovementComponent|SetMaxWalkSpeed (Variables|Character|GetCharacterMovement) 9e+02)))
  (:Released
    (Variables|Default|SetbRunning false)
    (Variables|/Script/Engine.CharacterMovementComponent|SetMaxWalkSpeed (Variables|Character|GetCharacterMovement) 5.5e+02)))

(event Input|ActionEvents|InputActionJump
  (params (Key :type Key%20Structure :default "None"))
  ;[1 1 1] Jumping
  (:Pressed
    (if (not (Variables|Default|GetbIsArmed))
      (Character|Jump)
      (Variables|Default|SetbInAir true))))

(event Input|AxisEvents|InputAxisWalkLeft/Right
  (params (AxisValue :type Float%20%28single-precision%29))
  ;[1 1 1] Movement
  (if (and (!= AxisValue 0.0) (not (Variables|Default|GetbIsAttacking)))
    (Pawn|Input|AddMovementInput (Math|Vector|GetRightVector (Math|Rotator|MakeRotator 0.0 0.0 (.yaw (Pawn|GetControlRotation :!class /Script/Engine.Pawn)))) AxisValue false)
    (Transformation|SetActorRotation (Math|Rotator|MakeRotator 0.0 0.0 (.yaw (Math|Conversions|RotationFromXVector (Variables|/Script/Engine.MovementComponent|GetVelocity (Variables|Character|GetCharacterMovement))))))
    (Class|AISenseHearing|ReportNoiseEvent (Transformation|GetActorLocation) 1.0 self 5e+02 "None")))

(event Input|AxisEvents|InputAxisWalkForward/Backward
  (params (AxisValue :type Float%20%28single-precision%29))
  ;[1 1 1] Movement
  (if (and (!= AxisValue 0.0) (not (Variables|Default|GetbIsAttacking)))
    (Pawn|Input|AddMovementInput (Math|Vector|GetForwardVector (Math|Rotator|MakeRotator 0.0 0.0 (.yaw (Pawn|GetControlRotation :!class /Script/Engine.Pawn)))) AxisValue false)
    (Transformation|SetActorRotation (Math|Rotator|MakeRotator 0.0 0.0 (.yaw (Math|Conversions|RotationFromXVector (Variables|/Script/Engine.MovementComponent|GetVelocity (Variables|Character|GetCharacterMovement))))))
    (Class|AISenseHearing|ReportNoiseEvent (Transformation|GetActorLocation) 1.0 self 5e+02 "None")))

(event Input|AxisEvents|InputAxisLookUp/Down
  (params (AxisValue :type Float%20%28single-precision%29))
  ;[1 1 1] Camera
  (Pawn|Input|AddControllerPitchInput AxisValue))

(event Input|AxisEvents|InputAxisLookLeft/Right
  (params (AxisValue :type Float%20%28single-precision%29))
  ;[1 1 1] Camera
  (Pawn|Input|AddControllerYawInput AxisValue))

(event Input|KeyboardEvents|I
  (params (Key :type Key%20Structure :default "None"))
  (bind _skeletalmesh (Variables|Default|GetSkeletalMesh))
  (bind _returnvalue (Transformation|GetSocketTransform _skeletalmesh "Weapon" "RTS_World"))
  ;[1 1 1] Equip/Unequip Weapon
  (:Pressed
    (Actor|DestroyActor (Variables|Default|GetWeaponRef))
    (Utilities|FlowControl|FlipFlop
      (:A
        (Variables|Default|SetbIsArmed true)
        (bind _returnvalue_2 (Game|SpawnActorfromClass "/Game/Objects/Weapons/Knife/Knife.Knife_C" _returnvalue "Undefined" 0 0))
        (Variables|Default|SetWeaponRef _returnvalue_2))
      (:B
        (Variables|Default|SetbIsArmed false)
        (bind _returnvalue_3 (Game|SpawnActorfromClass "/Game/Objects/Weapons/Fist/Punch.Punch_C" _returnvalue "Undefined" 0 0))
        (Variables|Default|SetWeaponRef _returnvalue_3)))
    (CallFunction|AttachWeapon)))

(fn ConstructionScript
  (Transformation|AttachComponentToComponent (Variables|Default|GetHeadHitBox) (Variables|Default|GetSkeletalMesh) "Head" "KeepRelative" "KeepRelative" "KeepRelative" true)
  (Transformation|AttachComponentToComponent (Variables|Default|GetBodyHitBox) (Variables|Default|GetSkeletalMesh) "Spine1" "KeepRelative" "KeepRelative" "KeepRelative" true))

(fn RotateifNeeded
  (bind _overlappedactor (Variables|Default|GetOverlappedActor))
  (bind _asnpc_bp (Utilities|Casting|CastToNPC_BP _overlappedactor))
  (if (Class|PrimitiveComponent|IsOverlappingComponent (Variables|Default|GetCapsuleComponent) (Variables|/Game/Humans/NPC/NPC_BP.NPC_BP_C|GetAttackArea _asnpc_bp))
    (Transformation|SetActorRelativeRotation self (Math|Rotator|MakeRotationfromAxes (- (Transformation|GetActorLocation _overlappedactor) (Transformation|GetActorLocation)) "0, 0, 0" "0, 0, 0"))))

(fn Die
  (Components|Movement|StopMovementImmediately (Variables|Character|GetCharacterMovement))
  (Actor|SetLifeSpan 8.0)
  (|CallParentFunction))