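; Human NPC character that wanders the navmesh, attacks a given victim and dies.
; A Move macro sends it to random reachable points after random delays, and overlapping another NPC or a door's collision turns it around.
; While moving it reports noise for AI hearing each tick.
; Construction attaches head and body hit boxes to skeleton sockets and sets stats text; Attack faces the victim and plays a montage.
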(event OnComponentBeginOverlap(CapsuleComponent)
  (params (OverlappedComponent :type Primitive%20Component%20Object%20Reference) (OtherActor :type Actor%20Object%20Reference) (OtherComp :type Primitive%20Component%20Object%20Reference) (OtherBodyIndex :type Integer) (bFromSweep :type Boolean) (SweepResult :type Hit%20Result%20Structure%20%28by%20ref%29))
  (Utilities|Casting|CastToNPC_BP OtherActor
    (:then
      (CallFunction|Rotate180))
    (:CastFailed
      (bind _asdoor_base (Utilities|Casting|CastToDoorBase OtherActor))
      (if (== (Variables|/Game/Objects/Architecture/door/DoorBase.DoorBase_C|Getcollision _asdoor_base) OtherComp)
        (CallFunction|Rotate180)))))

(event EventTick
  (params (DeltaSeconds :type Float%20%28single-precision%29))
  ;[1 1 1] Every Frame
  (if (Math|Vector|NotEqual(Vector) (Variables|/Script/Engine.MovementComponent|GetVelocity (Variables|Character|GetCharacterMovement)) "0, 0, 0" 0.01)
    (Class|AISenseHearing|ReportNoiseEvent (Transformation|GetActorLocation) 2.0 self 5e+02 "None")))

(fn ConstructionScript
  (Utilities|FlowControl|Sequence
    (:then_0
      (Transformation|AttachComponentToComponent (Variables|Default|GetHeadHitBox) (Variables|Default|GetSkeletalMesh) "Head" "KeepRelative" "KeepRelative" "KeepRelative" true)
      (Transformation|AttachComponentToComponent (Variables|Default|GetBodyHitBox) (Variables|Default|GetSkeletalMesh) "Spine1" "KeepRelative" "KeepRelative" "KeepRelative" true))
    (:then_1
      (Rendering|Components|TextRender|SetText (Variables|Default|GetStats) (Variables|Default|GetStatsTxt))
      (Rendering|Components|TextRender|SetTextRenderColor (Variables|Default|GetStats) (Math|Color|MakeColor 10 10 100)))))

(fn Die
  (Pawn|Components|CharacterMovement|DisableMovement (Variables|Character|GetCharacterMovement))
  (Collision|SetCollisionResponsetoAllChannels (Variables|Default|GetCapsuleComponent) "ECR_Ignore")
  (Components|Animation|PlayAnimation (Variables|Default|GetSkeletalMesh) "/Game/Humans/NPC/Animations/Dying_remy.Dying_remy" false)
  (Actor|SetLifeSpan 1e+01))

(fn Rotate180
  (bind _returnvalue (Transformation|GetActorRotation))
  (bind _charactermovement (Variables|Character|GetCharacterMovement))
  (switch Utilities|FlowControl|Switch|SwitchonEMovementMode (Variables|/Script/Engine.CharacterMovementComponent|GetMovementMode _charactermovement)
    (:MOVE_Walking
      _)
    (:MOVE_NavWalking
      _))
  (Class|NavMovementComponent|StopActiveMovement _charactermovement)
  (Transformation|SetActorRelativeRotation (Math|Rotator|MakeRotator (.roll _returnvalue) (.pitch _returnvalue) (+ (.yaw _returnvalue) 1.8e+02))))

(fn Attack
  (params (Victim :type Actor%20Object%20Reference))
  (Transformation|SetActorRotation (Math|Conversions|RotationFromXVector (- (Transformation|GetActorLocation Victim) (Transformation|GetActorLocation))))
  (Animation|Montage|MontagePlay (Components|SkeletalMesh|GetAnimInstance (Variables|Default|GetSkeletalMesh)) "/Game/Humans/NPC/Animations/RemyAttackM.RemyAttackM" 1.0 "MontageLength" 0.0 true)
  (return))