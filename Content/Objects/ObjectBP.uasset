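; Breakable world object that takes damage when something overlaps its Bounds.
; On overlap it flags its own data bitmask and queries DamageSystemHandler, which returns whether to continue, plus damage, effects and weapon owner.
; AddEffects decodes the effects bitmask per enum entry to decide if this hit can break it.
; If breakable at zero life or below, it expires after a short lifespan and increments the weapon owner's kill streak.
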(event OnComponentBeginOverlap(Bounds)
  (params (OverlappedComponent :type Primitive%20Component%20Object%20Reference) (OtherActor :type Actor%20Object%20Reference) (OtherComp :type Primitive%20Component%20Object%20Reference) (OtherBodyIndex :type Integer) (bFromSweep :type Boolean) (SweepResult :type Hit%20Result%20Structure%20%28by%20ref%29))
  (Variables|Default|SetSelfData (Class|KismetMathLibrary|OrIntInt (Variables|Default|GetSelfData) (|BitmaskLiteral 32)))
  (bind (_shouldcontinue _damage _effects _weaponowner) (Class|DamageSystem|DamageLogic(Message) (Variables|Default|GetDamageSystemHandler) self (Variables|Default|GetSelfData) OtherActor))
  (if _shouldcontinue
    (Variables|Default|SetWeaponOwner _weaponowner)
    (CallFunction|AddEffects _effects)
    (CallFunction|SetLife _damage)
    (if (and (Variables|Default|GetcanBreak) (<= (Variables|Default|GetLife) 0.0))
      (CallFunction|Die)
      (Utilities|IsValid (Variables|Default|GetWeaponOwner)
        (:Is%20Valid
          (Variables|/Game/Humans/Human.Human_C|SetKillStreak (Variables|Default|GetWeaponOwner) (+ (Variables|/Game/Humans/Human.Human_C|GetKillStreak (Variables|Default|GetWeaponOwner)) 1)))))))

(fn ConstructionScript)

(fn SetLife
  (params (Damage :type Float%20%28single-precision%29))
  (Variables|Default|SetLife (- (Variables|Default|GetLife) Damage)))

(fn Die
  (Actor|SetLifeSpan 3.0))

(fn AddEffects
  (params (Effects :type Integer))
  (Variables|Default|SetcanBreak false)
  (bind _enumvalue (|ForEachEEffects)
    (:LoopBody
      (if (Math|Conversions|ToBoolean(Integer) (Class|KismetMathLibrary|AndIntInt Effects (Math|Float|Floor (Math|Float|Power 2.0 (Math|Conversions|ToFloat(Byte) _enumvalue)))))
        (switch Utilities|FlowControl|Switch|SwitchonEEffects _enumvalue
          (:NewEnumerator3
            (Variables|Default|SetcanBreak true)))))))