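; Player character for a maze game with stealth enemies, handling movement, camera, HUD and a pause menu.
; Input feeds a movement component for walking, sprinting and crouching, which also changes walking loudness, while attack hold time is passed to an empty Attack stub.
; DamageSystem events reduce health; zero health or being seen by a stealth enemy destroys the character and reloads through the game mode.
; Construction attaches hit-zone components to mesh sockets.
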(event Custom|OnDie
  (bind _outactors (Actor|GetAllActorsOfClass "/Game/Character/Enemies/BP_StealthEnemy.BP_StealthEnemy_C"))
  (EventDispatchers|UnbindEventfromSeesPlayer _outactors (delegate Custom|OnDie))
  (Input|DisableInput (Game|GetPlayerController 0))
  (Utilities|FlowControl|Delay 1.5)
  (Actor|DestroyActor)
  (bind _ascustom_game_mode (Utilities|Casting|CastToCustomGameMode (Game|GetGameMode)))
  (Default|LoadGame _ascustom_game_mode))

(event Custom|Continue
  (bind _returnvalue (Game|GetPlayerController 0))
  (bind _menu (Variables|Default|GetMenu))
  (bind _hud (Variables|Default|GetHUD))
  (if (not (Variables|/Script/Engine.PlayerController|GetbShowMouseCursor (Game|GetPlayerController 0)))
    (UserInterface|Viewport|AddtoViewport _menu 0)
    (Variables|/Script/Engine.PlayerController|SetbShowMouseCursor _returnvalue true)
    (Input|SetInputModeGameandUI _returnvalue 0 "DoNotLock" true)
    (Widget|SetVisibility _hud "Hidden")
    (Game|SetGamePaused true)
    (else
      (Widget|RemovefromParent _menu)
      (Variables|/Script/Engine.PlayerController|SetbShowMouseCursor _returnvalue false)
      (Input|SetInputModeGameOnly _returnvalue)
      (Widget|SetVisibility _hud "Visible")
      (Game|SetGamePaused false))))

(event Custom|UpdateHealth
  (params (Damage :type Float%20%28single-precision%29))
  (CallFunction|UpdateHealthFunc Damage))

(event EventBeginPlay
  (bind _returnvalue (UserInterface|CreateWidget "/Game/UI/HUD.HUD_C"))
  (bind _output_get (Variables|Default|SetHUD _returnvalue))
  (UserInterface|Viewport|AddtoViewport _output_get 0)
  (bind _returnvalue_2 (UserInterface|CreateWidget "/Game/UI/PauseMenu.PauseMenu_C"))
  (Variables|Default|SetMenu _returnvalue_2)
  (Input|SetInputModeGameOnly (Game|GetPlayerController 0))
  (EventDispatchers|BindEventtoContinue (Variables|Default|GetMenu) (delegate Custom|Continue))
  (EventDispatchers|BindEventtoDamageProcessed (Variables|Default|GetDamageSystem) (delegate Custom|UpdateHealth))
  (bind _outactors (Actor|GetAllActorsOfClass "/Game/Character/Enemies/BP_StealthEnemy.BP_StealthEnemy_C"))
  (EventDispatchers|BindEventtoSeesPlayer _outactors (delegate Custom|OnDie))
  (EventDispatchers|BindEventtoDie (delegate Custom|OnDie)))

(event Input|ActionEvents|InputActionJump
  (params (Key :type Key%20Structure :default "None"))
  ;[1 1 1] For now, Unreal provided mechanics
  (:Pressed
    (Character|Jump))
  (:Released
    (Character|StopJumping)))

(event Input|ActionEvents|InputActionSprint
  (params (Key :type Key%20Structure :default "None"))
  (bind _movementcomp (Variables|Default|GetMovementComp))
  ;[1 1 1] Custom sprint logic
  (:Pressed
    (Variables|/Game/Character/MazeCharacter/MovementComp.MovementComp_C|SetbShiftDown _movementcomp true))
  (:Released
    (Variables|/Game/Character/MazeCharacter/MovementComp.MovementComp_C|SetbShiftDown _movementcomp false)))

(event Input|ActionEvents|InputActionCrouch
  (params (Key :type Key%20Structure :default "None"))
  (bind _movementcomp (Variables|Default|GetMovementComp))
  ;[1 1 1] For now, Unreal provided mechanics
  (:Pressed
    (Character|Crouch)
    (Variables|/Game/Character/MazeCharacter/MovementComp.MovementComp_C|SetbIsCrouched _movementcomp true)
    (Variables|/Game/Character/MazeCharacter/MovementComp.MovementComp_C|SetWalkingLoudness _movementcomp 1.0))
  (:Released
    (Character|UnCrouch)
    (Variables|/Game/Character/MazeCharacter/MovementComp.MovementComp_C|SetbIsCrouched _movementcomp false)
    (Variables|/Game/Character/MazeCharacter/MovementComp.MovementComp_C|SetWalkingLoudness _movementcomp 2.0)))

(event Input|ActionEvents|InputActionAttack
  (params (Key :type Key%20Structure :default "None"))
  (:Pressed
    (Class|KismetAnimationLibrary|StartProfilingTimer))
  (:Released
    (bind _returnvalue (Class|KismetAnimationLibrary|EndProfilingTimer false))
    (CallFunction|Attack _returnvalue)))

(event Input|AxisEvents|InputAxisWalkForward/Backward
  (params (AxisValue :type Float%20%28single-precision%29))
  ;[1 1 1] Movement
  (Default|MoveForward/Back (Variables|Default|GetMovementComp) AxisValue))

(event Input|AxisEvents|InputAxisWalkLeft/Right
  (params (AxisValue :type Float%20%28single-precision%29))
  ;[1 1 1] Movement
  (Default|MoveLeft/Right (Variables|Default|GetMovementComp) AxisValue))

(event Input|AxisEvents|InputAxisLookUp/Down
  (params (AxisValue :type Float%20%28single-precision%29))
  ;[1 1 1] Camera Control
  (Pawn|Input|AddControllerPitchInput AxisValue))

(event Input|AxisEvents|InputAxisLookLeft/Right
  (params (AxisValue :type Float%20%28single-precision%29))
  ;[1 1 1] Camera Control
  (Pawn|Input|AddControllerYawInput AxisValue))

(event Input|KeyboardEvents|M
  (params (Key :type Key%20Structure :default "None"))
  (bind _returnvalue (Game|GetPlayerController 0))
  (bind _menu (Variables|Default|GetMenu))
  (bind _hud (Variables|Default|GetHUD))
  (:Pressed
    (if (not (Variables|/Script/Engine.PlayerController|GetbShowMouseCursor (Game|GetPlayerController 0)))
      (UserInterface|Viewport|AddtoViewport _menu 0)
      (Variables|/Script/Engine.PlayerController|SetbShowMouseCursor _returnvalue true)
      (Input|SetInputModeGameandUI _returnvalue 0 "DoNotLock" true)
      (Widget|SetVisibility _hud "Hidden")
      (Game|SetGamePaused true)
      (else
        (Widget|RemovefromParent _menu)
        (Variables|/Script/Engine.PlayerController|SetbShowMouseCursor _returnvalue false)
        (Input|SetInputModeGameOnly _returnvalue)
        (Widget|SetVisibility _hud "Visible")
        (Game|SetGamePaused false)))))

(event Input|KeyboardEvents|Escape
  (params (Key :type Key%20Structure :default "None"))
  (bind _returnvalue (Game|GetPlayerController 0))
  (bind _menu (Variables|Default|GetMenu))
  (bind _hud (Variables|Default|GetHUD))
  (:Pressed
    (if (not (Variables|/Script/Engine.PlayerController|GetbShowMouseCursor (Game|GetPlayerController 0)))
      (UserInterface|Viewport|AddtoViewport _menu 0)
      (Variables|/Script/Engine.PlayerController|SetbShowMouseCursor _returnvalue true)
      (Input|SetInputModeGameandUI _returnvalue 0 "DoNotLock" true)
      (Widget|SetVisibility _hud "Hidden")
      (Game|SetGamePaused true)
      (else
        (Widget|RemovefromParent _menu)
        (Variables|/Script/Engine.PlayerController|SetbShowMouseCursor _returnvalue false)
        (Input|SetInputModeGameOnly _returnvalue)
        (Widget|SetVisibility _hud "Visible")
        (Game|SetGamePaused false)))))

(fn ConstructionScript
  (Transformation|AttachComponentToComponent (Variables|Default|GetHeadHZ) (Variables|Character|GetMesh) "Head" "KeepRelative" "KeepRelative" "KeepRelative" true)
  (Transformation|AttachComponentToComponent (Variables|Default|GetBodyHZ) (Variables|Character|GetMesh) "Spine" "KeepRelative" "KeepRelative" "KeepRelative" true)
  (Transformation|AttachComponentToComponent (Variables|Default|GetLArmHZ) (Variables|Character|GetMesh) "LeftArm" "KeepRelative" "KeepRelative" "KeepRelative" true)
  (Transformation|AttachComponentToComponent (Variables|Default|GetRArmHZ) (Variables|Character|GetMesh) "RightArm" "KeepRelative" "KeepRelative" "KeepRelative" true))

(fn UpdateHealthFunc
  (params (Damage :type Float%20%28single-precision%29))
  (bind _statscomp (Variables|Default|GetStatsComp))
  (bind _output_get (Variables|/Game/Character/MazeCharacter/StatsComp.StatsComp_C|SetHealth _statscomp (- (Variables|/Game/Character/MazeCharacter/StatsComp.StatsComp_C|GetHealth _statscomp) Damage)))
  (Default|CallHealthUpdated _output_get)
  (if (<= (Variables|/Game/Character/MazeCharacter/StatsComp.StatsComp_C|GetHealth (Variables|Default|GetStatsComp)) 0.0)
    (Default|CallDie)))

(fn Attack
  (params (Time :type Float%20%28single-precision%29)))