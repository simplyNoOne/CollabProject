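; Combat enemy character that makes melee attacks, takes damage and reports its death.
; Hit-zone components attach to head, spine and arm sockets, and an optional weapon spawns on the mesh.
; Attack yaws toward the target and plays a random montage from an armed or unarmed set.
; DamageSystem events stun it and reduce health; at zero it unequips, destroys non-Weapon items, unbinds and expires shortly after.
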(event Custom|OnDamaged
  (params (Damage :type Float%20%28single-precision%29))
  (bind _statscomp (Variables|Default|GetStatsComp))
  (bind _weapon (Variables|Default|GetWeapon))
  (Variables|Default|SetbIsStunned true)
  (Variables|/Game/Character/MazeCharacter/StatsComp.StatsComp_C|SetHealth _statscomp (- (Variables|/Game/Character/MazeCharacter/StatsComp.StatsComp_C|GetHealth _statscomp) Damage))
  (if (<= (Variables|/Game/Character/MazeCharacter/StatsComp.StatsComp_C|GetHealth (Variables|Default|GetStatsComp)) 0.0)
    (Utilities|IsValid _weapon
      (:Is%20Valid
        (Variables|/Game/Items/InteractiveItem.InteractiveItem_C|SetbIsEquipped _weapon false)
        (Utilities|Casting|CastToWeapon _weapon
          (:then
            _)
          (:CastFailed
            (Actor|DestroyActor _weapon))))
      (:Is%20Not%20Valid
        _))
    (EventDispatchers|UnbindallEventsfromDamageProcessed (Variables|Default|GetDamageSystem))
    (Actor|SetLifeSpan 1.0)
    (Default|CallEnemyDied)))

(event EventBeginPlay
  (if (Variables|Default|GetbSelectWeapon)
    (CallFunction|SpawnWeapon))
  (EventDispatchers|BindEventtoDamageProcessed (Variables|Default|GetDamageSystem) (delegate Custom|OnDamaged)))

(fn ConstructionScript
  (|CallParentFunction)
  (Transformation|AttachComponentToComponent (Variables|Default|GetHeadHZ) (Variables|Character|GetMesh) "Head" "KeepRelative" "KeepRelative" "KeepRelative" true)
  (Transformation|AttachComponentToComponent (Variables|Default|GetBodyHZ) (Variables|Character|GetMesh) "Spine" "KeepRelative" "KeepRelative" "KeepRelative" true)
  (Transformation|AttachComponentToComponent (Variables|Default|GetLArmHZ) (Variables|Character|GetMesh) "LeftArm" "KeepRelative" "KeepRelative" "KeepRelative" true)
  (Transformation|AttachComponentToComponent (Variables|Default|GetRArmHZ) (Variables|Character|GetMesh) "RightArm" "KeepRelative" "KeepRelative" "KeepRelative" true))

(fn Attack
  (params (AttackTarget :type Actor%20Object%20Reference))
  (Utilities|IsValid AttackTarget
    (:Is%20Valid
      (Transformation|SetActorRotation (Math|Rotator|MakeRotator 0.0 0.0 (.yaw (Math|Rotator|FindLookatRotation (Transformation|GetActorLocation) (Transformation|GetActorLocation AttackTarget)))))
      (if (Variables|Default|GetbIsArmed)
        (Animation|PlayAnimMontage (Utilities|Select :Index (Math|Random|RandomInteger 2) :Option%200 "/Game/Character/MazeCharacter/Anims/Attacks/Mannequin_Stabbing1_Montage.Mannequin_Stabbing1_Montage" :Option%201 "/Game/Character/MazeCharacter/Anims/Attacks/Mannequin_Standing_Melee_Punch_Montage.Mannequin_Standing_Melee_Punch_Montage") 1.0 "None")
        (else
          (Animation|PlayAnimMontage (Utilities|Select :Index (Math|Random|RandomInteger 3) :Option%200 "/Game/Character/MazeCharacter/Anims/Attacks/Manneequin_Elbow_Uppercut_Combo_Montage.Manneequin_Elbow_Uppercut_Combo_Montage" :Option%201 "/Game/Character/MazeCharacter/Anims/Attacks/Mannequin_Cross_Punch_Montage.Mannequin_Cross_Punch_Montage" :Option%202 "/Game/Character/MazeCharacter/Anims/Attacks/Mannequin_Standing_Melee_Punch_Montage.Mannequin_Standing_Melee_Punch_Montage") 1.0 "None"))))))

(fn SpawnWeapon
  (bind _returnvalue (Game|SpawnActorfromClass (Variables|Default|GetWeaponClass) (Transformation|GetActorTransform) "Undefined" 0 0))
  (bind _output_get (Variables|Default|SetWeapon _returnvalue))
  (Variables|/Game/Items/InteractiveItem.InteractiveItem_C|SetbIsEquipped _output_get true)
  (Default|SetCollision _output_get false)
  (Utilities|Casting|CastToWeapon _output_get
    (:then
      (Variables|Default|SetbIsArmed true))
    (:CastFailed
      _))
  (Transformation|AttachComponentToComponent (Variables|Default|GetWeapon) (Variables|Character|GetMesh) "MainSocket" "SnapToTarget" "SnapToTarget" "SnapToTarget" true))