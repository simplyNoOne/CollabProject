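; Enemy Blueprint that sets up body-part HZ components and provides a placeholder attack.
; The Construction Script runs the parent script, then attaches the head, body, left arm and right arm HZ components to matching Mesh sockets, keeping relative transforms.
; Attack ignores its target and only prints a brief red debug taunt.
; The event graph holds no active logic.
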(event EventBeginPlay)

(event Collision|EventActorBeginOverlap
  (params (OtherActor :type Actor%20Object%20Reference)))

(event EventTick
  (params (DeltaSeconds :type Float%20%28single-precision%29)))

(fn ConstructionScript
  (|CallParentFunction)
  (Transformation|AttachComponentToComponent (Variables|Default|GetHeadHZ) (Variables|Character|GetMesh) "Head" "KeepRelative" "KeepRelative" "KeepRelative" true)
  (Transformation|AttachComponentToComponent (Variables|Default|GetBodyHZ) (Variables|Character|GetMesh) "Spine" "KeepRelative" "KeepRelative" "KeepRelative" true)
  (Transformation|AttachComponentToComponent (Variables|Default|GetLArmHZ) (Variables|Character|GetMesh) "LeftArm" "KeepRelative" "KeepRelative" "KeepRelative" true)
  (Transformation|AttachComponentToComponent (Variables|Default|GetRArmHZ) (Variables|Character|GetMesh) "RightArm" "KeepRelative" "KeepRelative" "KeepRelative" true))

(fn Attack
  (params (AttackTarget :type Actor%20Object%20Reference))
  (Development|PrintString "DIE SCUM!" true true "(R=0.413542,G=0.007883,B=0.000000,A=1.000000)" 0.02))